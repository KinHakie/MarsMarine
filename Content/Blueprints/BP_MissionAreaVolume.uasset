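; BP_MissionAreaVolume is a boundary volume that punishes the player for leaving the mission area.
; When a BP_Marine exits the MissionArea component, it flags the marine as outside and starts a KillPlayer timer lasting SecondsBeforePlayerDeath.
; Re-entry clears the flag and timer.
; On expiry, KillPlayer applies heavy fixed damage to player character 0, regardless of which marine left.
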(event `self.MissionArea.OnComponentBeginOverlap`
  (params (OverlappedComponent :type "PrimitiveComponent Object Reference") (OtherActor :type "Actor Object Reference") (OtherComp :type "PrimitiveComponent Object Reference") (OtherBodyIndex :type Integer) (bFromSweep :type Boolean) (SweepResult :type "HitResult Structure (by ref)"))
  (bind _asbp_marine (cast `/Game/Blueprints/Pawns/BP_Marine` OtherActor))
  (set `/Game/Blueprints/Pawns/BP_Marine.OutsideMissionArea` false _asbp_marine)
  (`KismetSystemLibrary.K2_ClearTimer` null "KillPlayer"))

(event `self.MissionArea.OnComponentEndOverlap`
  (params (OverlappedComponent :type "PrimitiveComponent Object Reference") (OtherActor :type "Actor Object Reference") (OtherComp :type "PrimitiveComponent Object Reference") (OtherBodyIndex :type Integer))
  (bind _asbp_marine (cast `/Game/Blueprints/Pawns/BP_Marine` OtherActor))
  (set `/Game/Blueprints/Pawns/BP_Marine.OutsideMissionArea` true _asbp_marine)
  (`KismetSystemLibrary.K2_SetTimer` null "KillPlayer" (`self.SecondsBeforePlayerDeath`)))

(fn `KillPlayer`
  (`GameplayStatics.ApplyDamage` (`GameplayStatics.GetPlayerCharacter` 0) 100.0))

(fn `UserConstructionScript`)